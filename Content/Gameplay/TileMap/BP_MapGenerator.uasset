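; Tile map generator actor that builds a biome map on BeginPlay and renders it to render targets.
; After GenerateMap and DrawToRT, delayed material passes fill RT_BiomeCopy, then RT_BiomeNB.
; Tick steps the sample X and Y together, wrapped by map size, and prints the biome there as debug output.
; A color tileset render pass is present but unconnected.
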(event EventBeginPlay
  (Utilities|FlowControl|Sequence
    (:then_1
      (Class|MapGenerator|GenerateMap)
      (Class|MapGenerator|DrawtoRT)
      (Utilities|FlowControl|Delay 1.0)
      (Rendering|DrawMaterialtoRenderTarget "/Game/Gameplay/TileMap/RT_BiomeCopy.RT_BiomeCopy" "/Game/Gameplay/TileMap/M_CopyRT.M_CopyRT")
      (Utilities|FlowControl|Delay 1.0)
      (Rendering|DrawMaterialtoRenderTarget "/Game/Gameplay/TileMap/Neighbor/RT_BiomeNB.RT_BiomeNB" "/Game/Gameplay/TileMap/Neighbor/M_BiomeNB.M_BiomeNB"))))

(event Collision|EventActorBeginOverlap
  (params (OtherActor :type Actor%20Object%20Reference)))

(event EventTick
  (params (DeltaSeconds :type Float%20%28single-precision%29))
  (bind _returnvalue (Class|MapGenerator|GetBiomeatLocation (Variables|Default|Getix) (Variables|Default|Getiy)))
  (Development|PrintText (Utilities|Text|FormatText "TileX : {0} , TileX :{1} , Boime : {2}" (Variables|Default|Getix) (Variables|Default|Getiy) (|GenerictoText _returnvalue)))
  (Variables|Default|Setix (Math|Integer|%(Integer) (+ (Variables|Default|Getix) 4) (Math|Float|Truncate (Variables|Default|GetMapWidth))))
  (Variables|Default|Setiy (Math|Integer|%(Integer) (+ (Variables|Default|Getiy) 4) (Math|Float|Truncate (Variables|Default|GetMapHeight)))))

(fn ConstructionScript)